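; Player-controlled Paper2D character that moves along the world X and Z axes from two input axes, with a Parar flag that zeroes movement.
; Each Tick, SetMyFlipbook stores the last input direction, vertical taking priority, and selects one of four directional flipbooks for the sprite.
; On BeginPlay it clears Parar and moves the first Spawner actor to the Localização saved in the controladorGeral GameInstance.
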(event EventBeginPlay
  (Variables|Default|Setparar false)
  (Development|PrintString "Hello")
  (bind _outactors (Actor|GetAllActorsOfClass "/Game/Blueprints/Spawner.Spawner_C"))
  (bind _ascontrolador_geral (Utilities|Casting|CastTocontroladorGeral (Game|GetGameInstance)))
  (Transformation|SetActorLocation (Utilities|Array|Get(acopy) _outactors) (Variables|/Game/Blueprints/controladorGeral.controladorGeral_C|Getlocalização _ascontrolador_geral) false false))

(event EventTick
  (params (DeltaSeconds :type Float%20%28single-precision%29))
  (CallFunction|SetMyFlipbook))

(event Input|AxisEvents|InputAxisCimaOuBaixo
  (params (AxisValue :type Float%20%28single-precision%29))
  (if (Variables|Default|Getparar)
    (Pawn|Input|AddMovementInput "0, 0, 0" AxisValue false)
    (else
      (Pawn|Input|AddMovementInput "0.0,0.0,1.0" AxisValue false))))

(event Input|AxisEvents|InputAxisEsquerdaOuDireita
  (params (AxisValue :type Float%20%28single-precision%29))
  (if (Variables|Default|Getparar)
    (Pawn|Input|AddMovementInput "0, 0, 0" AxisValue false)
    (else
      (Pawn|Input|AddMovementInput "1.000000, 0,0.000000" AxisValue false))))

(fn ConstructionScript)

(fn SetMyFlipbook
  (if (or (!= (Input|AxisValues|GetEsquerdaOuDireita) 0.0) (!= (Input|AxisValues|GetCimaOuBaixo) 0.0))
    (Variables|Default|SetLastMoveDirection (select (> (Input|AxisValues|GetCimaOuBaixo) 0.0) "NewEnumerator0" (select (< (Input|AxisValues|GetCimaOuBaixo) 0.0) "NewEnumerator1" (select (> (Input|AxisValues|GetEsquerdaOuDireita) 0.0) "NewEnumerator3" "NewEnumerator2")))))
  (Sprite|SetFlipbook (Variables|Default|GetSprite) (select (> (Math|Vector|VectorLength (Transformation|GetVelocity)) 0.0) (Utilities|Select :Index (Variables|Default|GetLastMoveDirection) :NewEnumerator0 "/Game/Texturas/cima_Flipbook.cima_Flipbook" :NewEnumerator1 "/Game/Texturas/baixo_Flipbook.baixo_Flipbook" :NewEnumerator2 "/Game/Texturas/esquerda_Flipbook.esquerda_Flipbook" :NewEnumerator3 "/Game/Texturas/direita_Flipbook.direita_Flipbook") (Utilities|Select :Index (Variables|Default|GetLastMoveDirection) :NewEnumerator0 "/Game/Texturas/cima_Flipbook.cima_Flipbook" :NewEnumerator1 "/Game/Texturas/baixo_Flipbook.baixo_Flipbook" :NewEnumerator2 "/Game/Texturas/esquerda_Flipbook.esquerda_Flipbook" :NewEnumerator3 "/Game/Texturas/direita_Flipbook.direita_Flipbook"))))